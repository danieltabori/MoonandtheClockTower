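; Player character that steps through scenes of eight locations, such as Beach, Museum and Old Town, shown in an outdoor scenes widget created on BeginPlay.
; GetSceneLineNumber stores the chosen scene line and resets the scene index to 1.
; Previous and Next inputs move the index and update the widget, stopping at zero and at per-line limits from SceneLocationMaxRule.
; A similar SceneLocationNumberMaxRules function is unused here and differs on line 4.
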(event `self.ReceiveBeginPlay`
  ;[0 1 0] Creates Widget With Scenes
  (bind _returnvalue (`|CreateWidget` "/Game/Blueprints/Widget_blueprints/WB_Scenes/WB_Outdoors_Scenes.WB_Outdoors_Scenes_C"))
  (set `self.WB_Outdoors` _returnvalue)
  (`UserWidget.AddToViewport` _returnvalue 0)
  (`/Game/Blueprints/Widget_blueprints/WB_Scenes/WB_Outdoors_Scenes.ChangeLocation` (`self.WB_Outdoors`) (`self.SceneLocation`)))

(event `InputAction|Previous Scene`
  (params (Key :type "Key Structure"))
  ;[0 1 0] Moves Backwards
  (:`Pressed`
    (if (not (== (`self.SceneLocation`) 0))
      (`/Engine/EditorBlueprintResources/StandardMacros.DecrementInt` (`self.SceneLocation`)
        (:`  `
          (`/Game/Blueprints/Widget_blueprints/WB_Scenes/WB_Outdoors_Scenes.ChangeLocation` (`self.WB_Outdoors`) (`self.SceneLocation`)))))))

(event `InputAction|Next Scene`
  (params (Key :type "Key Structure"))
  ;[0 1 0] Moves Forward
  (:`Pressed`
    (`self.SceneLocationMaxRule`
      (:`Beach`
        _)
      (:`StudentDorm`
        _)
      (:`Hospital`
        _)
      (:`Museum`
        _)
      (:`FamillyHouse`
        _)
      (:`RooftopBar`
        _)
      (:`OldTown`
        _)
      (:`FortressWalls`
        _))
    (`/Engine/EditorBlueprintResources/StandardMacros.IncrementInt` (`self.SceneLocation`)
      (:`  `
        (`/Game/Blueprints/Widget_blueprints/WB_Scenes/WB_Outdoors_Scenes.ChangeLocation` (`self.WB_Outdoors`) (`self.SceneLocation`))))))

(event `/Game/Blueprints/Blueprint_Interfaces/BPI_Player_Map_Communication.GetSceneLineNumber`
  (params (SceneLine :type Integer))
  ;[0 1 0] Player_Character Recieves information about direction of our movement
  (set `self.SceneLine` SceneLine)
  (set `self.SceneLocation` 1))

(fn `SceneLocationNumberMaxRules`
  (switch `int` (`self.SceneLine`)
    (:`1`
      (if (not (== (`self.SceneLocation`) 1))
        (return)))
    (:`2`
      (if (not (== (`self.SceneLocation`) 2))
        (return)))
    (:`3`
      (if (not (== (`self.SceneLocation`) 1))
        (return)))
    (:`4`
      (if (not (== (`self.SceneLocation`) 3))
        (return)))
    (:`5`
      (if (not (== (`self.SceneLocation`) 2))
        (return)))
    (:`6`
      (if (not (== (`self.SceneLocation`) 1))
        (return)))
    (:`7`
      (if (not (== (`self.SceneLocation`) 4))
        (return)))
    (:`8`
      (if (not (== (`self.SceneLocation`) 3))
        (return)))))

(fn `UserConstructionScript`)